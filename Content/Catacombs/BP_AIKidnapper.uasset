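; BP_AIKidnapper is a Catacombs AI character with Walk to, Patrol and Chase behaviors, selected by a fixed switch at BeginPlay.
; Each uses AI MoveTo: walking from cell to crypt target, looping through patrol points, or chasing the player until a "GAME OVER" print.
; The switch input is a constant zero rather than a variable, so behavior never changes at runtime.
; Pawn sensing only prints a guard-signal message.
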(event OnSeePawn(PawnSensing)
  (params (Pawn :type Pawn%20Object%20Reference))
  (Development|PrintString "Signal to guards"))

(event Custom|WalkTo
  (AI|AIMoveTo self "0, 0, 0" (Variables|Default|GetCellTarget) 5.0 false
    (:OnSuccess
      (Utilities|FlowControl|Delay 1.0)
      (AI|AIMoveTo self "0, 0, 0" (Variables|Default|GetCryptTarget) 5.0 false))))

(event Custom|Patrol%20To%20Point
  (AI|AIMoveTo self "0, 0, 0" (Utilities|Array|Get(acopy) (Variables|Default|GetPatrolPoints) (Variables|Default|GetPatrolPointIndex)) 5.0 false
    (:OnSuccess
      (if (>= (Variables|Default|GetPatrolPointIndex) (- (Utilities|Array|Length (Variables|Default|GetPatrolPoints)) 1))
        (Variables|Default|SetPatrolPointIndex 0)
        (else
          (Math|Integer|IncrementInt (Variables|Default|GetPatrolPointIndex)
            (:%20%20
              _))))
      (CallFunction|PatroltoPoint))))

(event Custom|Chase%20Player
  (AI|AIMoveTo self "0, 0, 0" (Game|GetPlayerCharacter 0) 5.0 false
    (:OnSuccess
      (Development|PrintString "GAME OVER"))))

(event EventBeginPlay
  (switch Utilities|FlowControl|Switch|Switchon 0
    (:NewEnumerator0
      (CallFunction|Walkto))
    (:NewEnumerator1
      (CallFunction|PatroltoPoint))
    (:NewEnumerator2
      (CallFunction|ChasePlayer))))

(fn ConstructionScript)