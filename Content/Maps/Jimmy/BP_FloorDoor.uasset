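; BP_FloorDoor is a floor door actor that swings open once when interacted with.
; Overlaps on InteractionBox with the FirstPersonCharacter toggle CanBeOpened, which gates the Interact event.
; Interact clears that flag and calls OpenDoor, which sets DoorOpened and plays a timeline driving the Door's relative roll.
; The Fire input handler checks both flags but performs no action, and nothing closes the door.
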(event OnComponentBeginOverlap(InteractionBox)
  (params (OverlappedComponent :type Primitive%20Component%20Object%20Reference) (OtherActor :type Actor%20Object%20Reference) (OtherComp :type Primitive%20Component%20Object%20Reference) (OtherBodyIndex :type Integer) (bFromSweep :type Boolean) (SweepResult :type Hit%20Result%20Structure%20%28by%20ref%29))
  (Utilities|Casting|CastToFirstPersonCharacter OtherActor)
  (Variables|Default|SetCanBeOpened true))

(event OnComponentEndOverlap(InteractionBox)
  (params (OverlappedComponent :type Primitive%20Component%20Object%20Reference) (OtherActor :type Actor%20Object%20Reference) (OtherComp :type Primitive%20Component%20Object%20Reference) (OtherBodyIndex :type Integer))
  (Utilities|Casting|CastToFirstPersonCharacter OtherActor)
  (Variables|Default|SetCanBeOpened false))

(event Custom|OpenDoor
  (Variables|Default|SetDoorOpened true)
  (bind _doorangle (Timeline|Timeline_Door Play)
    (:Update
      (Transformation|SetRelativeRotation (Variables|Default|GetDoor) (Math|Rotator|MakeRotator _doorangle 0.0 0.0) false false))))

(event EventBeginPlay)

(event Collision|EventActorBeginOverlap
  (params (OtherActor :type Actor%20Object%20Reference)))

(event EventInteract
  (if (Variables|Default|GetCanBeOpened)
    (Variables|Default|SetCanBeOpened false)
    (CallFunction|OpenDoor)))

(event EventTick
  (params (DeltaSeconds :type Float%20%28single-precision%29)))

(event Input|ActionEvents|InputActionFire
  (params (Key :type Key%20Structure))
  (:Pressed
    (if (not (Variables|Default|GetDoorOpened))
      (if (Variables|Default|GetCanBeOpened)
        _))))

(fn ConstructionScript)